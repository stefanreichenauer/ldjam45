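; Player character Blueprint with axis-driven movement and look, a charge-based jump, and a toggleable double jump.
; Jumping launches the character upward and spends a charge, which landing restores to the maximum.
; The skill tree input toggles pause, the WT_SkillTree widget, cursor and input mode, passing the character to the widget.
; ToggleDoubleJump switches the maximum between one and two jumps, refilling charges unless flying.
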(event Custom|ToggleDoubleJump
  (params (bIsDoubleJumpActive :type Boolean))
  (bind _charactermovement (Variables|Character|GetCharacterMovement))
  (bind _returnvalue (Class|NavMovementComponent|IsFlying _charactermovement))
  (bind _output_get (Variables|Default|SetbIsDoubleJumpingActive bIsDoubleJumpActive))
  (if _output_get
    (bind _output_get_2 (Variables|Default|SetMaxNumberOfJumps 2))
    (if (not _returnvalue)
      (Variables|Default|SetCurrentNumberOfJumps _output_get_2))
    (else
      (bind _output_get_3 (Variables|Default|SetMaxNumberOfJumps 1))
      (if (not _returnvalue)
        (Variables|Default|SetCurrentNumberOfJumps _output_get_3)))))

(event EventOnLanded
  (params (Hit :type Hit%20Result%20Structure%20%28by%20ref%29))
  (Variables|Default|SetCurrentNumberOfJumps (Variables|Default|GetMaxNumberOfJumps)))

(event Input|ActionEvents|InputActionJump
  (params (Key :type Key%20Structure :default "None"))
  (:Pressed
    (if (> (Variables|Default|GetCurrentNumberOfJumps) 0)
      (Character|LaunchCharacter "0, 0,1000.000000" false false)
      (Math|Integer|DecrementInt (Variables|Default|GetCurrentNumberOfJumps)))))

(event Input|ActionEvents|InputActionOpenSkilltree
  (params (Key :type Key%20Structure :default "None"))
  (bind _returnvalue (Game|GetPlayerController 0))
  (bind _returnvalue_2 (Game|GetPlayerController 0))
  (:Pressed
    (if (Variables|Default|GetIsGamePaused)
      (Game|SetGamePaused false)
      (Viewport|RemoveAllWidgets)
      (Input|SetInputModeGameOnly _returnvalue)
      (Variables|/Script/Engine.PlayerController|SetbShowMouseCursor _returnvalue false)
      (Variables|Default|SetIsGamePaused false)
      (else
        (Game|SetGamePaused true)
        (bind _returnvalue_3 (UserInterface|CreateWidget "/Game/Widgets/WT_SkillTree.WT_SkillTree_C"))
        (UserInterface|Viewport|AddtoViewport _returnvalue_3 0)
        (Default|InitializeSkilltree _returnvalue_3 self)
        (Input|SetInputModeGameandUI _returnvalue_2 _returnvalue_3 "DoNotLock" true)
        (Variables|/Script/Engine.PlayerController|SetbShowMouseCursor _returnvalue_2 true)
        (Variables|Default|SetIsGamePaused true)))))

(event Input|AxisEvents|InputAxisTurn
  (params (AxisValue :type Float%20%28single-precision%29))
  (Pawn|Input|AddControllerYawInput AxisValue))

(event Input|AxisEvents|InputAxisLookUp
  (params (AxisValue :type Float%20%28single-precision%29))
  (Pawn|Input|AddControllerPitchInput AxisValue))

(event Input|AxisEvents|InputAxisMoveForward
  (params (AxisValue :type Float%20%28single-precision%29))
  (Pawn|Input|AddMovementInput (Transformation|GetActorForwardVector) AxisValue false))

(event Input|AxisEvents|InputAxisMoveRight
  (params (AxisValue :type Float%20%28single-precision%29))
  (Pawn|Input|AddMovementInput (Transformation|GetActorRightVector) AxisValue false))

(fn ConstructionScript)